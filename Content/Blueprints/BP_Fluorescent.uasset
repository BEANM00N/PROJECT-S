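; BP_Fluorescent is a configurable fluorescent light fixture made of a main mesh, two wing meshes and a rect light.
; The construction script sets the meshes' mobility and rolls the left and right wings by separate angles, mirrored for the left side.
; It then applies exposed settings to the rect light, covering brightness, radius, source size, scattering, shadows, mobility and color.
; The event graph is empty, so the fixture has no runtime logic.
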(fn `UserConstructionScript`
  (bind _sm_fluorescent_wings_right (`self.SM_Fluorescent_Wings_Right`))
  (bind _rectlight (`self.RectLight`))
  (`SceneComponent.SetMobility` _sm_fluorescent_wings_right (`self.Light Mesh Mobility`))
  (`SceneComponent.SetMobility` (`self.SM_Fluorescent_Wings_Left`) (`self.Light Mesh Mobility`))
  (`SceneComponent.SetMobility` (`self.SM_Fluorescent`) (`self.Light Mesh Mobility`))
  (`|ExecutionSequence`
    (:`then_0`
      (`SceneComponent.K2_AddLocalTransform` _sm_fluorescent_wings_right (`KismetMathLibrary.MakeTransform` (0.0 0.0 0.0) (`KismetMathLibrary.MakeRotator` (`self.Right Wing Angle`))) false false))
    (:`then_1`
      (`SceneComponent.K2_AddLocalTransform` (`self.SM_Fluorescent_Wings_Left`) (`KismetMathLibrary.MakeTransform` (0.0 0.0 0.0) (`KismetMathLibrary.MakeRotator` (* (`self.Left Wing Angle`) -1.0))) false false))
    (:`then_2`
      (`LightComponent.SetIntensity` _rectlight (`self.Light Intensity`))
      (`LocalLightComponent.SetAttenuationRadius` _rectlight (`self.Light Radius`))
      (`RectLightComponent.SetSourceHeight` _rectlight (`self.Source Height`))
      (`RectLightComponent.SetSourceWidth` _rectlight (`self.Source Width`))
      (`LightComponent.SetIndirectLightingIntensity` _rectlight (`self.Light Indirect Intensity`))
      (`LightComponent.SetVolumetricScatteringIntensity` _rectlight (`self.Light Volumetric Scattering Intensity`))
      (`LightComponentBase.SetCastShadows` _rectlight (`self.Cast Shadow`))
      (`SceneComponent.SetMobility` _rectlight (`self.Light Mobility`))
      (`LightComponent.SetLightColor` _rectlight (`self.Color`) true))))